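; Intruder variant Blueprint that supplies the character's surprised voice reaction through a PlaySound function.
; PlaySound picks randomly among three Surprised sounds and plays one at the capsule's location, louder and higher-pitched than normal.
; The random range has four outcomes, so one in four calls plays nothing.
; The event graph holds only disabled placeholder events, and the construction script just calls its parent.
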(event EventBeginPlay
  (|CallParentFunction) ; This node is disabled and will not be called.\nDrag off pins to build functionality.
)

(event Collision|EventActorBeginOverlap
  (params (OtherActor :type Actor%20Object%20Reference)))

(event EventTick
  (params (DeltaSeconds :type Float%20%28single-precision%29)))

(fn ConstructionScript
  (|CallParentFunction))

(fn PlaySound
  (bind _capsulecomponent (Variables|Default|GetCapsuleComponent))
  (bind _returnvalue (Transformation|GetWorldLocation _capsulecomponent))
  (switch int (Math|Random|RandomInteger 4)
    (:0
      (Audio|PlaySoundatLocation "/Game/Sounds/FX/surprised.surprised" _returnvalue "0, 0, 0" 2.0 1.5 0.0 0 0 0))
    (:1
      (Audio|PlaySoundatLocation "/Game/Sounds/FX/surprised_b.surprised_b" _returnvalue "0, 0, 0" 2.0 1.5 0.0 0 0 0))
    (:2
      (Audio|PlaySoundatLocation "/Game/Sounds/FX/surprised_c.surprised_c" _returnvalue "0, 0, 0" 2.0 1.5 0.0 0 0 0))))