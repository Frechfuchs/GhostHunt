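; Intruder character that wanders, notices player-controlled possessable pawns and can be spooked or scared to death.
; Box overlaps switch a string State, stop movement on sighting and randomly play a surprise sound.
; Helper functions handle head look-at rotation, wait timers, walk/run speed, sanity and fleeing from a spook location.
; The level's exit is cached at BeginPlay; no state update loop runs in this graph.
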(event OnComponentBeginOverlap(Box)
  (params (OverlappedComponent :type Primitive%20Component%20Object%20Reference) (OtherActor :type Actor%20Object%20Reference) (OtherComp :type Primitive%20Component%20Object%20Reference) (OtherBodyIndex :type Integer) (bFromSweep :type Boolean) (SweepResult :type Hit%20Result%20Structure%20%28by%20ref%29))
  ;[1 1 1] Seeing Possessable
  (bind _asbp_possesable_pawn (Utilities|Casting|CastToBP_PossesablePawn OtherActor))
  (if (Class|Pawn|IsControlled _asbp_possesable_pawn)
    (Variables|Default|SetPossessableToLookAt _asbp_possesable_pawn)
    (Variables|Default|SetState "LOOKAT")
    (Class|NavMovementComponent|StopActiveMovement (Variables|Character|GetCharacterMovement))
    (CallFunction|PlaySound)))

(event OnComponentEndOverlap(Box)
  (params (OverlappedComponent :type Primitive%20Component%20Object%20Reference) (OtherActor :type Actor%20Object%20Reference) (OtherComp :type Primitive%20Component%20Object%20Reference) (OtherBodyIndex :type Integer))
  ;[1 1 1] Seeing Possessable
  (if (== OtherActor (Variables|Default|GetPossessableToLookAt))
    (Variables|Default|SetState "LOSTLOOKAT")
    (CallFunction|UnsetPossessabletoLookat)))

(event EventSpookfromLocation
  (params (Location :type Vector :default "0, 0, 0"))
  ;[1 1 1] Spooked from Location
  (CallFunction|SetupSpookedfromLocation Location))

(event EventBeginPlay
  ;[1 1 1] Find Exit
  (bind _returnvalue (Actor|GetActorOfClass "/Game/Blueprints/BP_IntruderExit.BP_IntruderExit_C"))
  (Variables|Default|SetExitPoint _returnvalue))

(fn ConstructionScript)

(fn LookatPossessablePawn
  (bind _possessabletolookat (Variables|Default|GetPossessableToLookAt))
  (bind _debugarrow (Variables|Default|GetDebugArrow))
  (bind _returnvalue (Transformation|GetWorldLocation _debugarrow))
  (bind _staticmesh (Variables|/Game/Blueprints/Possessables/BP_PossesablePawn.BP_PossesablePawn_C|GetStaticMesh _possessabletolookat))
  (bind _returnvalue_2 (Transformation|GetWorldLocation _staticmesh))
  (bind _returnvalue_3 (Math|Rotator|FindLookatRotation _returnvalue _returnvalue_2))
  (Variables|Default|SetHeadRotation (Math|Rotator|MakeRotator (* (.pitch _returnvalue_3) -1.0) 0.0 (- (.yaw _returnvalue_3) (.yaw (Transformation|GetWorldRotation (Variables|Default|GetDebugArrow)))))))

(fn ResetRotation
  (Variables|Default|SetHeadRotation (Math|Rotator|MakeRotator 0.0 0.0 0.0))
  (return))

(fn ResetState
  (Variables|Default|SetState "WANDERAROUND")
  (return))

(fn UpdateWaitingTimeDelta
  (params (DeltaSeconds :type Float%20%28single-precision%29))
  (bind _output_get (Variables|Default|SetWaitingTime (- (Variables|Default|GetWaitingTime) DeltaSeconds)))
  (return (<= _output_get 0.0)))

(fn SetupWaiting
  (params (WaitingTime :type Float%20%28single-precision%29))
  (Variables|Default|SetWaitingTime WaitingTime)
  (Variables|Default|SetState "WAITING")
  (return))

(fn ResetWaiting
  (Variables|Default|SetWaitingTime 0.0)
  (return))

(fn CheckPossessableIsControlled
  (return (Class|Pawn|IsControlled (Variables|Default|GetPossessableToLookAt))))

(fn SetupLookatUnpossessedPawn
  (Variables|Default|SetWaitingTime 4.0)
  (Variables|Default|SetState "LOOKATUNPOSSESSED")
  (return))

(fn UnsetPossessabletoLookat
  (Variables|Default|SetPossessableToLookAt 0))

(fn Run
  (Utilities|IsValid self
    (:Is%20Valid
      (Variables|/Script/Engine.CharacterMovementComponent|SetMaxWalkSpeed (Variables|Character|GetCharacterMovement) (Variables|Default|GetRunSpeed))
      (return))))

(fn Walk
  (Variables|/Script/Engine.CharacterMovementComponent|SetMaxWalkSpeed (Variables|Character|GetCharacterMovement) (Variables|Default|GetWalkSpeed))
  (return))

(fn SetupSpookedfromLocation
  (params (From :type Vector))
  (Class|NavMovementComponent|StopActiveMovement (Variables|Character|GetCharacterMovement))
  (CallFunction|Run)
  (Variables|Default|SetTargetLocation (* (Math|Vector|GetUnitDirection(Vector) From (Transformation|GetWorldLocation (Variables|Collision|GetCapsuleComponent))) 4e+02))
  (Variables|Default|SetState "SPOOKEDFROMLOCATION"))

(fn Turn180
  (bind _capsulecomponent (Variables|Collision|GetCapsuleComponent))
  (Transformation|SetWorldRotation _capsulecomponent (Math|Rotator|MakeRotator 0.0 0.0 (+ (.yaw (Transformation|GetWorldRotation _capsulecomponent)) 1.8e+02)) false false)
  (return))

(fn CheckScaredtoDeath
  (if (<= (Variables|Default|GetSanity) 0)
    (Variables|Default|SetState "SCAREDTODEATH"))
  (return))

(fn UpdateSanity
  (params (AddedSanity :type Integer))
  (Variables|Default|SetSanity (+ AddedSanity (Variables|Default|GetSanity)))
  (return))

(fn PlaySound
  (bind _capsulecomponent (Variables|Collision|GetCapsuleComponent))
  (bind _returnvalue (Transformation|GetWorldLocation _capsulecomponent))
  (switch int (Math|Random|RandomInteger 4)
    (:0
      (Audio|PlaySoundatLocation "/Game/Sounds/FX/surprised.surprised" _returnvalue "0, 0, 0" 2.0 1.0 0.0 0 0 0))
    (:1
      (Audio|PlaySoundatLocation "/Game/Sounds/FX/surprised_b.surprised_b" _returnvalue "0, 0, 0" 2.0 1.0 0.0 0 0 0))
    (:2
      (Audio|PlaySoundatLocation "/Game/Sounds/FX/surprised_c.surprised_c" _returnvalue "0, 0, 0" 2.0 1.0 0.0 0 0 0))))