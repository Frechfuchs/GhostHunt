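; Player controller that sets up the player's HUD and keeps a reference to the BP_Ghost pawn.
; On BeginPlay it creates and displays WBP_PlayerHUD, then casts player pawn 0 to BP_Ghost and stores it through the SetGhostPawn event.
; When the Debugging flag is set it also creates a debug widget and adds it to the viewport, but only if that cast succeeds.
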(event Custom|SetGhostPawn
  (params (GhostPawn :type BP%20Ghost%20Object%20Reference))
  ;[1 1 1] Register Ghost Pawn
  (Variables|Default|SetGhost%20Pawn GhostPawn))

(event EventBeginPlay
  ;[1 1 1] Add HUD
  (bind _returnvalue (UserInterface|CreateWidget "/Game/Blueprints/Widgets/WBP_PlayerHUD.WBP_PlayerHUD_C"))
  (bind _output_get (Variables|Default|SetPlayerHUD _returnvalue))
  (UserInterface|Viewport|AddtoViewport _output_get 0)
  (bind _asbp_ghost (Utilities|Casting|CastToBP_Ghost (Game|Player|GetPlayerPawn 0)))
  (CallFunction|SetGhostPawn _asbp_ghost)
  ;;[1 0.8688 0] DEBUGGING ONLY
  (if (Variables|Debug|GetDebugging)
    (bind _returnvalue_2 (UserInterface|CreateWidget "/Game/Blueprints/Widgets/WBP_Debugging.WBP_Debugging_C"))
    (bind _output_get_2 (Variables|Debug|SetDebugHUD _returnvalue_2))
    (UserInterface|Viewport|AddtoViewport _output_get_2 0)))

(fn ConstructionScript)