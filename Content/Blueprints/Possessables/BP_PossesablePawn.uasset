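; Base pawn for a physics object that the player's ghost can possess and fly around for a limited time.
; Possessing disables gravity, raises damping and starts a HUD countdown, while camera-relative forces on the static mesh drive movement.
; Timeout or Interact restores gravity and returns control to the ghost pawn, teleported to the camera.
; Focus toggles a custom-depth stencil highlight, and an uncalled helper randomly plays spook sounds.
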(event Custom|Unpossess
  (bind _camera (Variables|Default|GetCamera))
  (bind _playercontroller (Variables|Default|GetPlayerController))
  (bind _ghost_pawn (Variables|/Game/Blueprints/BP_PlayerController.BP_PlayerController_C|GetGhost%20Pawn _playercontroller))
  ;[1 1 1] Unpossess this pawn
  (Transformation|Teleport (Variables|/Game/Blueprints/BP_PlayerController.BP_PlayerController_C|GetGhost%20Pawn (Variables|Default|GetPlayerController)) (Transformation|GetWorldLocation _camera) (Transformation|GetWorldRotation _camera))
  (CallFunction|StopPossessTimer)
  (Pawn|Possess _playercontroller _ghost_pawn)
  (Variables|/Game/Blueprints/BP_Ghost.BP_Ghost_C|SetIsPossessed _ghost_pawn true)
  (Physics|SetEnableGravity (Variables|Default|GetStaticMesh) true)
  (Class|PrimitiveComponent|SetLinearDamping (Variables|Default|GetStaticMesh) 0.01))

(event EventBeginPlay
  ;[1 1 1] Set simulate physics on
  (Physics|SetEnableGravity (Variables|Default|GetStaticMesh) (Variables|Default|GetStartGravityEnabled)))

(event EventTick
  (params (DeltaSeconds :type Float%20%28single-precision%29))
  ;[1 1 1] PossessTimer
  (if (Variables|Default|GetPossessStarted)
    (bind _output_get (Variables|Default|SetPossessTimeLeft (- (Variables|Default|GetPossessTimeLeft) DeltaSeconds)))
    (if (<= _output_get 0.0)
      (CallFunction|Unpossess)
      (else
        (CallFunction|UpdatePossessTimer)))))

(event EventStartFocus
  ;[1 1 1] Handle Focus
  (Rendering|SetCustomDepthStencilValue (Variables|Default|GetStaticMesh) 252)
  (Rendering|SetRenderCustomDepth (Variables|Default|GetStaticMesh) true))

(event EventPossess
  ;[1 1 1] On Possess
  (Rendering|SetRenderCustomDepth (Variables|Default|GetStaticMesh) false)
  (bind _asbp_player_controller (Utilities|Casting|CastToBP_PlayerController (Game|GetPlayerController 0)))
  (bind _output_get (Variables|Default|SetPlayerController _asbp_player_controller))
  (bind _output_get_2 (Variables|Default|SetPlayer%20HUD (Variables|/Game/Blueprints/BP_PlayerController.BP_PlayerController_C|GetPlayerHUD _output_get)))
  (Default|ShowUnPossessPrompt _output_get_2)
  (Physics|SetEnableGravity (Variables|Default|GetStaticMesh) false)
  (Class|PrimitiveComponent|SetLinearDamping (Variables|Default|GetStaticMesh) 15.0)
  (CallFunction|StartPossessTimer))

(event EventEndFocus
  ;[1 1 1] Handle Focus
  (Rendering|SetRenderCustomDepth (Variables|Default|GetStaticMesh) false))

(event Input|ActionEvents|InputActionInteract
  (params (Key :type Key%20Structure :default "None"))
  ;[1 1 1] Unpossess this pawn
  (:Pressed
    (CallFunction|Unpossess)))

(event Input|AxisEvents|InputAxisMoveForward
  (params (AxisValue :type Float%20%28single-precision%29))
  ;[1 1 1] Movement
  (Physics|AddForce (Variables|Default|GetStaticMesh) (* (* (Math|Vector|GetForwardVector (Variables|Default|GetCamera)) 5e+03) AxisValue) "None" true))

(event Input|AxisEvents|InputAxisMoveRight
  (params (AxisValue :type Float%20%28single-precision%29))
  ;[1 1 1] Movement
  (Physics|AddForce (Variables|Default|GetStaticMesh) (* (* (Math|Vector|GetRightVector (Variables|Default|GetCamera)) 5e+03) AxisValue) "None" true))

(event Input|AxisEvents|InputAxisTurnRate
  (params (AxisValue :type Float%20%28single-precision%29))
  ;[1 1 1] Look around Gamepad
  (Pawn|Input|AddControllerYawInput (* AxisValue (Variables|Default|GetBaseTurnRate) (Utilities|Time|GetWorldDeltaSeconds))))

(event Input|AxisEvents|InputAxisLookUpRate
  (params (AxisValue :type Float%20%28single-precision%29))
  ;[1 1 1] Look around Gamepad
  (Pawn|Input|AddControllerPitchInput (* AxisValue (Variables|Default|GetBaseLookUpRate) (Utilities|Time|GetWorldDeltaSeconds))))

(event Input|AxisEvents|InputAxisTurn
  (params (AxisValue :type Float%20%28single-precision%29))
  ;[1 1 1] Look around Mouse
  (Pawn|Input|AddControllerYawInput AxisValue))

(event Input|AxisEvents|InputAxisLookUp
  (params (AxisValue :type Float%20%28single-precision%29))
  ;[1 1 1] Look around Mouse
  (Pawn|Input|AddControllerPitchInput AxisValue))

(event Input|AxisEvents|InputAxisMoveUp
  (params (AxisValue :type Float%20%28single-precision%29))
  ;[1 1 1] Movement
  (Physics|AddForce (Variables|Default|GetStaticMesh) (* "0, 0,5000.000000" AxisValue) "None" true))

(fn ConstructionScript)

(fn StartPossessTimer
  (Variables|Default|SetPossessTimeLeft (Variables|Default|GetPossessTime))
  (Variables|Default|SetPossessStarted true)
  (Default|ShowProgressBar (Variables|Default|GetPlayer%20HUD))
  (return))

(fn UpdatePossessTimer
  (Default|UpdateProgress (Variables|Default|GetPlayer%20HUD) (/ (Variables|Default|GetPossessTimeLeft) (Variables|Default|GetPossessTime))))

(fn StopPossessTimer
  (Variables|Default|SetPossessStarted false)
  (Default|HideProgressBar (Variables|Default|GetPlayer%20HUD)))

(fn PlaySound
  (switch int (Math|Random|RandomInteger 8)
    (:0
      (Audio|PlaySound2D "/Game/Sounds/FX/spook.spook" 1.0 1.0 0.0 0 0))
    (:1
      (Audio|PlaySound2D "/Game/Sounds/FX/spook_b.spook_b" 1.0 1.0 0.0 0 0))
    (:2
      (Audio|PlaySound2D "/Game/Sounds/FX/spook_c.spook_c" 1.0 1.0 0.0 0 0))
    (:3
      (Audio|PlaySound2D "/Game/Sounds/FX/spook_d.spook_d" 1.0 1.0 0.0 0 0))))