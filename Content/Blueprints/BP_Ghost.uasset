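; BP_Ghost is the player's free-flying ghost pawn, which can use objects and possess other pawns.
; It registers with BP_PlayerController, takes its HUD, and handles camera-relative movement plus mouse and gamepad look.
; A camera line trace each Tick finds interactable or possessable actors, driving focus messages and HUD prompts while IsPossessed is true.
; Interact either uses the focused actor or blends the view to a BP_PossesablePawn, then possesses it.
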(event Custom|HandleLinetrace
  (params (HasHit :type Boolean) (HitActor :type Actor%20Object%20Reference))
  (bind _playerhud (Variables|Default|GetPlayerHUD))
  ;[1 1 1] Handle LineTrace HUD
  (if (Variables|Default|GetIsPossessed)
    (CallFunction|EndFocus)
    (if HasHit
      (bind _output_get (Variables|Default|SetFocusedActor HitActor))
      (if (Utilities|DoesObjectImplementInterface _output_get "/Game/Blueprints/BPI_Interactable.BPI_Interactable_C")
        (Default|ShowUsePrompt _playerhud)
        (else
          (Default|ShowPossessPrompt _playerhud)))
      (Class|BPIUsable|StartFocus(Message) (Variables|Default|GetFocusedActor))
      (else
        (Variables|Default|SetFocusedActor 0)
        (Default|HidePrompt (Variables|Default|GetPlayerHUD))))))

(event EventTick
  (params (DeltaSeconds :type Float%20%28single-precision%29))
  (bind _camera (Variables|Default|GetCamera))
  (bind _returnvalue (Transformation|GetWorldLocation _camera))
  ;[1 1 1] LineTrace
  (bind (_outhit _returnvalue_2) (Collision|LineTraceByChannel _returnvalue (+ _returnvalue (* (Math|Vector|GetForwardVector _camera) (Variables|Default|GetInteractRange))) "TraceTypeQuery2" false 0 "None"))
  (if _returnvalue_2
    (if (or (Utilities|DoesObjectImplementInterface (.HitActor (Collision|BreakHitResult _outhit)) "/Game/Blueprints/BPI_Interactable.BPI_Interactable_C") (Utilities|DoesObjectImplementInterface (.HitActor (Collision|BreakHitResult _outhit)) "/Game/Blueprints/BPI_Possesable.BPI_Possesable_C"))
      (CallFunction|HandleLinetrace true (.HitActor (Collision|BreakHitResult _outhit))))
    (else
      (CallFunction|HandleLinetrace false))))

(event EventBeginPlay
  ;[1 1 1] Get Player HUD
  (bind _asbp_player_controller (Utilities|Casting|CastToBP_PlayerController (Game|GetPlayerController 0)))
  (Utilities|IsValid (Variables|/Game/Blueprints/BP_PlayerController.BP_PlayerController_C|GetPlayerHUD _asbp_player_controller)
    (:Is%20Valid
      (Variables|Default|SetPlayerHUD (Variables|/Game/Blueprints/BP_PlayerController.BP_PlayerController_C|GetPlayerHUD _asbp_player_controller))
      (Default|SetGhostPawn _asbp_player_controller self))))

(event Input|ActionEvents|InputActionInteract
  (params (Key :type Key%20Structure :default "None"))
  (bind _returnvalue (Game|GetPlayerController 0))
  (bind _focusedactor (Variables|Default|GetFocusedActor))
  (bind _focusedactor_2 (Variables|Default|GetFocusedActor))
  ;[1 1 1] Use
  (:Pressed
    (Utilities|IsValid _focusedactor
      (:Is%20Valid
        (if (Utilities|DoesObjectImplementInterface _focusedactor "/Game/Blueprints/BPI_Interactable.BPI_Interactable_C")
          (Class|BPIInteractable|Use(Message) _focusedactor_2)
          (else
            (bind _asbp_possesable_pawn (Utilities|Casting|CastToBP_PossesablePawn _focusedactor_2))
            (Variables|Default|SetIsPossessed false)
            (Game|Player|SetViewTargetwithBlend _returnvalue _asbp_possesable_pawn 0.5 "VTBlend_Linear" 0.0 false)
            (Utilities|FlowControl|Delay 0.5)
            (Pawn|Possess _returnvalue _asbp_possesable_pawn)
            (Class|BPIPossesable|Possess(Message) _asbp_possesable_pawn)))))))

(event Input|AxisEvents|InputAxisMoveForward
  (params (AxisValue :type Float%20%28single-precision%29))
  ;[1 1 1] Movement
  (Pawn|Input|AddMovementInput (Math|Vector|GetForwardVector (Variables|Default|GetCamera)) AxisValue false))

(event Input|AxisEvents|InputAxisMoveRight
  (params (AxisValue :type Float%20%28single-precision%29))
  ;[1 1 1] Movement
  (Pawn|Input|AddMovementInput (Math|Vector|GetRightVector (Variables|Default|GetCamera)) AxisValue false))

(event Input|AxisEvents|InputAxisTurnRate
  (params (AxisValue :type Float%20%28single-precision%29))
  ;[1 1 1] Look around Gamepad
  (Pawn|Input|AddControllerYawInput (* AxisValue (Variables|Input|GetBaseTurnRate) (Utilities|Time|GetWorldDeltaSeconds))))

(event Input|AxisEvents|InputAxisLookUpRate
  (params (AxisValue :type Float%20%28single-precision%29))
  ;[1 1 1] Look around Gamepad
  (Pawn|Input|AddControllerPitchInput (* AxisValue (Variables|Input|GetBaseLookUpRate) (Utilities|Time|GetWorldDeltaSeconds))))

(event Input|AxisEvents|InputAxisTurn
  (params (AxisValue :type Float%20%28single-precision%29))
  ;[1 1 1] Look around Mouse
  (Pawn|Input|AddControllerYawInput AxisValue))

(event Input|AxisEvents|InputAxisLookUp
  (params (AxisValue :type Float%20%28single-precision%29))
  ;[1 1 1] Look around Mouse
  (Pawn|Input|AddControllerPitchInput AxisValue))

(event Input|AxisEvents|InputAxisMoveUp
  (params (AxisValue :type Float%20%28single-precision%29))
  ;[1 1 1] Movement
  (Pawn|Input|AddMovementInput (Math|Vector|GetUpVector (Variables|Default|GetSphere)) AxisValue false))

(fn ConstructionScript)

(fn EndFocus
  (bind _focusedactor (Variables|Default|GetFocusedActor))
  (Utilities|IsValid _focusedactor
    (:Is%20Valid
      (Class|BPIUsable|EndFocus(Message) _focusedactor))))