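; Base-style interactable actor that scares nearby pawns when used.
; Focus events toggle a custom depth stencil highlight on its static mesh.
; Use clears the highlight, calls an empty PlaySound stub, then runs a sphere overlap and sends a spook-from-location message to pawns implementing BPI_Scareable, passing the actor's root location.
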(event EventStartFocus
  ;[1 1 1] Handle Focus
  (Rendering|SetCustomDepthStencilValue (Variables|Default|GetStaticMesh) 252)
  (Rendering|SetRenderCustomDepth (Variables|Default|GetStaticMesh) true))

(event EventEndFocus
  ;[1 1 1] Handle Focus
  (Rendering|SetRenderCustomDepth (Variables|Default|GetStaticMesh) false))

(event EventUse
  ;[1 1 1] Scare on Use with Sphere Overlap
  (Rendering|SetRenderCustomDepth (Variables|Default|GetStaticMesh) false)
  (CallFunction|PlaySound (Transformation|GetWorldLocation (Variables|Default|GetDefaultSceneRoot)))
  (bind _outactors (Collision|SphereOverlapActors (Transformation|GetWorldLocation (Variables|Default|GetDefaultSceneRoot)) 5e+02 (Utilities|Array|MakeArray "ObjectTypeQuery3") 0))
  (for _array_element _outactors
    (if (Utilities|DoesObjectImplementInterface _array_element "/Game/Blueprints/BPI_Scareable.BPI_Scareable_C")
      (Class|BPIScareable|SpookfromLocation(Message) _array_element (Transformation|GetWorldLocation (Variables|Default|GetDefaultSceneRoot))))))

(fn ConstructionScript)

(fn PlaySound
  (params (Location :type Vector)))