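; Default game mode that runs the FirstFloor level's intruder count and ends the game when the last intruder leaves.
; On start it sets the count from LevelIndex, plays the theme music and caches the player HUD.
; IntruderLeft decrements the count and updates the HUD, or shows the game over widget before returning to Title.
; Intruder spawning at the BP_IntruderExit actor is defined, but the batch call is disconnected.
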(event Custom|PrepareLevel
  ;[1 1 1] Prepare Level
  (switch int (Variables|Default|GetLevelIndex)
    (:0
      (bind _intrudercount (CallFunction|LevelOne))
      (Variables|Default|SetIntruderCount _intrudercount)
      (Audio|PlaySound2D "/Game/Sounds/BG/Bonneton_Theme.Bonneton_Theme" 0.4 0.75 0.0 0 0))))

(event Custom|SpawnIntruders
  (params (IntruderCount :type Integer))
  ;[1 1 1] Spawn Batch of Intruders
  (bind _output_get (Variables|Default|SetIntruderCount IntruderCount))
  (for _index (range 1 _output_get)
    (CallFunction|SpawnIntruder)))

(event Custom|SpawnIntruder
  ;[1 1 1] Spawn Single Intruder
  (Game|SpawnActorfromClass "/Game/Blueprints/Intruder/BP_Intruder.BP_Intruder_C" (Transformation|GetActorTransform (Variables|Default|GetBP_IntruderExit)) "AdjustIfPossibleButAlwaysSpawn" 0 0))

(event Custom|IntruderLeft
  ;[1 1 1] Intruder left
  (bind _result (Math|Integer|DecrementInt (Variables|Default|GetIntruderCount))
    (:%20%20
      (if (<= _result 0)
        (CallFunction|GameOver)
        (else
          (CallFunction|UpdatePlayerHUDIntruders))))))

(event Custom|UpdatePlayerHUDIntruders
  (bind _playerhud (Variables|Default|GetPlayerHUD))
  ;[1 1 1] Update Intruder Count in Player HUD
  (Utilities|IsValid _playerhud
    (:Is%20Valid
      (Default|UpdateIntrudersCount _playerhud (Variables|Default|GetIntruderCount)))))

(event Custom|GameOver
  ;[1 1 1] Game over
  (Widget|RemovefromParent (Variables|Default|GetPlayerHUD))
  (bind _returnvalue (UserInterface|CreateWidget "/Game/Blueprints/Widgets/WBP_GameOver.WBP_GameOver_C" (Variables|Default|GetPlayerController)))
  (UserInterface|Viewport|AddtoViewport _returnvalue 0)
  (Utilities|FlowControl|Delay 8.0)
  (Game|OpenLevel(byName) "Title"))

(event EventBeginPlay
  ;[1 1 1] Init
  (bind _returnvalue (Actor|GetActorOfClass "/Game/Blueprints/BP_IntruderExit.BP_IntruderExit_C"))
  (Variables|Default|SetBP_IntruderExit _returnvalue)
  (bind _returnvalue_2 (Game|GetCurrentLevelName true))
  (if (Utilities|Enum|Equal(Enum) _returnvalue_2 "FirstFloor")
    (CallFunction|PrepareLevel)
    (Utilities|FlowControl|Delay 1.0)
    (bind _asbp_player_controller (Utilities|Casting|CastToBP_PlayerController (Game|GetPlayerController 0)))
    (bind _output_get (Variables|Default|SetPlayerController _asbp_player_controller))
    (Variables|Default|SetPlayerHUD (Variables|/Game/Blueprints/BP_PlayerController.BP_PlayerController_C|GetPlayerHUD _output_get))
    (CallFunction|UpdatePlayerHUDIntruders)))

(fn ConstructionScript)

(fn LevelOne
  (return (LocalVariables|GetLevelIntruderCount)))